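; Main player character Blueprint that handles the pause menu and quick save/load input.
; QuitToMenu shows the cursor, pauses the game and opens the PauseMenu widget.
; QuickSave has every SavableObject interface actor write into a new GameSaveData, saves it to a slot and prints a Polish success or failure message.
; QuickLoad reads that slot and passes the data back to those actors.
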(event `InputAction|QuitToMenu`
  (params (Key :type "Key Structure"))
  (:`Pressed`
    (set `PlayerController.bShowMouseCursor` true (`GameplayStatics.GetPlayerController` 0))
    (`GameplayStatics.SetGamePaused` true)
    (bind _returnvalue (`|CreateWidget` "/Game/Blueprints/UserInterface/Menus/GamePauseMenu/PauseMenu.PauseMenu_C"))
    (`UserWidget.AddToViewport` _returnvalue 0)))

(event `InputAction|QuickSave`
  (params (Key :type "Key Structure"))
  (:`Pressed`
    (bind _returnvalue (`GameplayStatics.CreateSaveGameObject` "/Script/HorrorGame.GameSaveData"))
    (bind _outactors (`GameplayStatics.GetAllActorsWithInterface` "/Script/HorrorGame.SavableObject"))
    (for _array_element _outactors
      (message `SavableObject.SaveDataToGameSave` _array_element _returnvalue))
    (bind _returnvalue_2 (`GameplayStatics.SaveGameToSlot` _returnvalue (`self.SaveName`)))
    (if _returnvalue_2
      (`KismetSystemLibrary.PrintString` "Zapis udany!" true true (struct :`G` 0.66 :`B` 1.0 :`A` 1.0) 5.0)
      (else
        (`KismetSystemLibrary.PrintString` "Niepowodzenie zapisu" true true (struct :`R` 1.0 :`B` 0.041948 :`A` 1.0) 5.0)))))

(event `InputAction|QuickLoad`
  (params (Key :type "Key Structure"))
  (:`Pressed`
    (bind _returnvalue (`GameplayStatics.LoadGameFromSlot` (`self.SaveName`)))
    (bind _asgame_save_data (cast `GameSaveData` _returnvalue))
    (bind _outactors (`GameplayStatics.GetAllActorsWithInterface` "/Script/HorrorGame.SavableObject"))
    (for _array_element _outactors
      (message `SavableObject.LoadDataFromGameSave` _array_element _asgame_save_data))))

(fn `UserConstructionScript`)