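; Base game mode Blueprint that applies saved game user settings and manages sound class volumes.
; On BeginPlay it loads and applies user settings, then sets the base sound mix.
; Volume events store values in SoundOptions and fade overrides onto the Music, Dialogue and Effects classes, each scaled by master volume.
; Master changes refresh all three; the Master class override receives no volume value of its own.
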(event `self.ReceiveBeginPlay`
  (bind _returnvalue (`GameUserSettings.GetGameUserSettings`))
  (`GameUserSettings.LoadSettings` _returnvalue false)
  (`GameUserSettings.ApplySettings` _returnvalue true)
  (`GameplayStatics.SetBaseSoundMix` "/Game/Blueprints/Sounds/SoundMix/BaseSoundMix.BaseSoundMix"))

(event `ChangeMasterVolume`
  (params (MasterVolume :type "Float (double-precision)"))
  (bind (_mastervolume _effectsvolume _musicvolume _dialoguevolume) (break `/Game/Blueprints/GameOptions/SoundOptions` (`self.SoundOptions`)))
  (`|VariableSetRef` _mastervolume MasterVolume)
  (`GameplayStatics.SetSoundMixClassOverride` "/Game/Blueprints/Sounds/SoundMix/BaseSoundMix.BaseSoundMix" "/Game/Blueprints/Sounds/SoundClasses/Master.Master" 1.0 1.0 0.2)
  (`|ExecutionSequence`
    (:`then_0`
      (`GameplayStatics.SetSoundMixClassOverride` "/Game/Blueprints/Sounds/SoundMix/BaseSoundMix.BaseSoundMix" "/Game/Blueprints/Sounds/SoundClasses/Music.Music" (* _musicvolume _mastervolume) 1.0 0.2 :!label _label))
    (:`then_1`
      (`GameplayStatics.SetSoundMixClassOverride` "/Game/Blueprints/Sounds/SoundMix/BaseSoundMix.BaseSoundMix" "/Game/Blueprints/Sounds/SoundClasses/Dialogue.Dialogue" (* _dialoguevolume _mastervolume) 1.0 0.2 :!label _label_2))
    (:`then_2`
      (`GameplayStatics.SetSoundMixClassOverride` "/Game/Blueprints/Sounds/SoundMix/BaseSoundMix.BaseSoundMix" "/Game/Blueprints/Sounds/SoundClasses/Effects.Effects" (* _effectsvolume _mastervolume) 1.0 0.2 :!label _label_3))))

(event `ChangeMusicVolume`
  (params (MusicVolume :type "Float (double-precision)"))
  (`|VariableSetRef` (`.MusicVolume_11_B7AD010B406EC65EFE91B79E72F40A6A` (break `/Game/Blueprints/GameOptions/SoundOptions` (`self.SoundOptions`))) MusicVolume)
  (goto _label))

(event `ChangeDialogueVolume`
  (params (DialogueVolume :type "Float (double-precision)"))
  (`|VariableSetRef` (`.DialogueVolume_12_F8B8AA8E468384B04E45A7B56022D56B` (break `/Game/Blueprints/GameOptions/SoundOptions` (`self.SoundOptions`))) DialogueVolume)
  (goto _label_2))

(event `ChangeEffectsVolume`
  (params (EffectsVolume :type "Float (double-precision)"))
  (`|VariableSetRef` (`.EffectsVolume_10_FFC16D2A4E1C12FFA85747BEA3869C3F` (break `/Game/Blueprints/GameOptions/SoundOptions` (`self.SoundOptions`))) EffectsVolume)
  (goto _label_3))

(fn `UserConstructionScript`)