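; Game instance that loads the player's audio and game user settings at startup and exposes volume controls.
; On Init it constructs an AudioUserSettings object from a base sound mix and Master, Music, Effects and Dialogue sound classes, then loads it and applies GameUserSettings.
; World changes and per-category volume events are forwarded to that audio settings object, which receives the new world context on each change.
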(event `self.ReceiveInit`
  ;[1 1 1] Audio User Settings
  (bind _returnvalue (`|GenericCreateObject` "/Script/HorrorGame.AudioUserSettings" self))
  (bind _output_get (set `self.AudioSettings` _returnvalue))
  (`AudioUserSettings.Init` _output_get "/Game/Blueprints/Sounds/SoundMix/BaseSoundMix.BaseSoundMix" (make `SoundClasses` "/Game/Blueprints/Sounds/SoundClasses/Master.Master" "/Game/Blueprints/Sounds/SoundClasses/Music.Music" "/Game/Blueprints/Sounds/SoundClasses/Effects.Effects" "/Game/Blueprints/Sounds/SoundClasses/Dialogue.Dialogue"))
  (`AudioUserSettings.LoadSettings` _output_get)
  ;[1 1 1] Game User Settings
  (bind _returnvalue_2 (`GameUserSettings.GetGameUserSettings`))
  (`GameUserSettings.LoadSettings` _returnvalue_2 false)
  (`GameUserSettings.ApplySettings` _returnvalue_2 true))

(event `OnWorldChanged`
  (params (WorldContextObject :type "Object Object Reference"))
  (bind _output_get (set `self.WorldContextObject` WorldContextObject))
  ;[1 1 1] Audio Managing
  (`AudioUserSettings.ChangeWorld` (`self.AudioSettings`) _output_get))

(event `ChangeMasterVolume`
  (params (MasterVolume :type "Float (double-precision)"))
  ;[1 1 1] Audio Managing
  (`AudioUserSettings.ChangeMasterVolume` (`self.AudioSettings`) MasterVolume))

(event `ChangeMusicVolume`
  (params (MusicVolume :type "Float (double-precision)"))
  ;[1 1 1] Audio Managing
  (`AudioUserSettings.ChangeMusicVolume` (`self.AudioSettings`) MusicVolume))

(event `ChangeDialogueVolume`
  (params (DialogueVolume :type "Float (double-precision)"))
  ;[1 1 1] Audio Managing
  (`AudioUserSettings.ChangeDialogueVolume` (`self.AudioSettings`) DialogueVolume))

(event `ChangeEffectsVolume`
  (params (EffectsVolume :type "Float (double-precision)"))
  ;[1 1 1] Audio Managing
  (`AudioUserSettings.ChangeEffectsVolume` (`self.AudioSettings`) EffectsVolume))